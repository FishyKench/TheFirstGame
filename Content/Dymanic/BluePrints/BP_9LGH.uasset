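; BP_9LGH is a trigger actor that gives the player a different melee weapon when its box is overlapped.
; The overlap event casts player character 0 to BP_Player without checking which actor overlapped.
; It then copies its weapon mesh and material onto the player's MeleeWeapon component and overwrites the player's attack range and weapon damage.
; The actor stays in place afterwards.
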(event `self.Box.OnComponentBeginOverlap`
  (params (OverlappedComponent :type "PrimitiveComponent Object Reference") (OtherActor :type "Actor Object Reference") (OtherComp :type "PrimitiveComponent Object Reference") (OtherBodyIndex :type Integer) (bFromSweep :type Boolean) (SweepResult :type "HitResult Structure (by ref)"))
  (bind _asbp_player (cast `/Game/Dymanic/BluePrints/BP_Player` (`GameplayStatics.GetPlayerCharacter` 0)))
  (bind _output_get (set `self.Player` _asbp_player))
  (`PrimitiveComponent.SetMaterial` (`/Game/Dymanic/BluePrints/BP_Player.MeleeWeapon` _output_get) 0 (`self.WeaponMaterial`))
  (`StaticMeshComponent.SetStaticMesh` (`/Game/Dymanic/BluePrints/BP_Player.MeleeWeapon` (`self.Player`)) (`self.WeaponStaticMesh`))
  (set `/Game/Dymanic/BluePrints/BP_Player.AttackRange` (`self.WeaponAttackRange`) (`self.Player`))
  (set `/Game/Dymanic/BluePrints/BP_Player.WeaponDamage` (`self.WeaponDamage`) (`self.Player`)))

(fn `UserConstructionScript`)