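; BP_BaseWeapon is a base weapon Blueprint that equips the player with its look and combat stats.
; On BeginPlay it casts player character 0 to BP_Player, then applies its static mesh and material to the player's MeleeWeapon component.
; It also copies its attack range and damage into the player's variables, holding only data and setup with no attack logic of its own.
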(event `self.ReceiveBeginPlay`
  (bind _asbp_player (cast `/Game/Dymanic/BluePrints/BP_Player` (`GameplayStatics.GetPlayerCharacter` 0)))
  (bind _output_get (set `self.Player` _asbp_player))
  (`PrimitiveComponent.SetMaterial` (`/Game/Dymanic/BluePrints/BP_Player.MeleeWeapon` _output_get) 0 (`self.WeaponMaterial`))
  (`StaticMeshComponent.SetStaticMesh` (`/Game/Dymanic/BluePrints/BP_Player.MeleeWeapon` (`self.Player`)) (`self.WeaponStaticMesh`))
  (set `/Game/Dymanic/BluePrints/BP_Player.AttackRange` (`self.WeaponAttackRange`) (`self.Player`))
  (set `/Game/Dymanic/BluePrints/BP_Player.WeaponDamage` (`self.WeaponDamage`) (`self.Player`)))

(fn `UserConstructionScript`)