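; BP_Base_Enemy is a base enemy character Blueprint providing a melee attack, patrol route access and movement speed control.
; Attack plays the machete light attack montage on the mesh and calls OnAttackEnd whether the montage completes or is interrupted.
; GetPatrolRoute exposes the assigned route, and SetMovementSpeed maps a speed state from idle to sprinting onto the CharacterMovement max walk speed and returns it.
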(event `self.ReceiveBeginPlay`)

(event `Attack`
  (`|PlayMontage` (`self.Mesh`) "/Game/MacheteAnimationPack/Animation/Animation_Montage/AM_Machete_LightAttack.AM_Machete_LightAttack"
    (:`OnCompleted`
      _)
    (:`OnInterrupted`
      _))
  (`self.OnAttackEnd`))

(fn `GetPatrolRoute`
  (returns (PatrolRoute :type "/Game/Dymanic/BluePrints/AI/BP_PatrolRoute Object Reference"))
  (return (`self.PatrolRoute`)))

(fn `SetMovementSpeed`
  (params (Speed :type "/Game/Dymanic/BluePrints/AI/Enums/E_MovementSpeed Enum" :default "NewEnumerator0"))
  (returns (SpeedValue :type "Float (double-precision)"))
  (bind _output_get (set `CharacterMovementComponent.MaxWalkSpeed` (select `/Game/Dymanic/BluePrints/AI/Enums/E_MovementSpeed` Speed :`NewEnumerator1` 100.0 :`NewEnumerator2` 300.0 :`NewEnumerator3` 500.0 :!type "Float (single-precision)") (`self.CharacterMovement`)))
  (return _output_get))

(fn `UserConstructionScript`)