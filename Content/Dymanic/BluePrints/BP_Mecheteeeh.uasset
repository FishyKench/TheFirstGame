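; BP_Mecheteeeh is a machete pickup that equips the player's melee weapon.
; On BeginPlay it casts the player character to BP_Player and caches the reference.
; When that player overlaps its Box, it swaps the MeleeWeapon mesh and material to the machete and overwrites the player's attack range and weapon damage.
; The actor neither destroys nor hides itself afterward, so each new overlap reapplies the same values.
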(event `self.ReceiveBeginPlay`
  (bind _asbp_player (cast `/Game/Dymanic/BluePrints/BP_Player` (`GameplayStatics.GetPlayerCharacter` 0)))
  (set `self.Player` _asbp_player))

(event `self.Box.OnComponentBeginOverlap`
  (params (OverlappedComponent :type "PrimitiveComponent Object Reference") (OtherActor :type "Actor Object Reference") (OtherComp :type "PrimitiveComponent Object Reference") (OtherBodyIndex :type Integer) (bFromSweep :type Boolean) (SweepResult :type "HitResult Structure (by ref)"))
  (bind _player (`self.Player`))
  (bind _meleeweapon (`/Game/Dymanic/BluePrints/BP_Player.MeleeWeapon` (`self.Player`)))
  (if (== OtherActor (`self.Player`))
    (`StaticMeshComponent.SetStaticMesh` _meleeweapon "/Game/MacheteAnimationPack/Meshes/SM_Machete.SM_Machete")
    (`PrimitiveComponent.SetMaterial` _meleeweapon 0 "/Game/MacheteAnimationPack/Material/Master/M_Machete.M_Machete")
    (set `/Game/Dymanic/BluePrints/BP_Player.AttackRange` 500.0 _player)
    (set `/Game/Dymanic/BluePrints/BP_Player.WeaponDamage` 50.0 _player)))

(fn `UserConstructionScript`)