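; BP_Enemy_Mage is an enemy mage Blueprint that fights at range by casting fireball spells at its target.
; Its Attack event plays a fireball montage, and a montage notify fires a damaging spell from the right hand socket through the BPCAttacks component.
; Montage completion or interruption clears the attacking state and signals attack end.
; It also supplies movement speeds per movement state and preferred attack and defend ranges.
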(event `/Game/Dymanic/BluePrints/Enemies/AI/BPI_EnemyAI.Attack`
  (params (AttackTarget :type "Actor Object Reference"))
  (bind _notifyname (`|PlayMontage` (`self.Mesh`) "/Game/Dymanic/Characters/Mage/Animations/Montages/Montage_Mage_Fireball.Montage_Mage_Fireball")
    (:`OnCompleted`
      (`self.OnAttackEnd` :!label _label)
      (set `self.Attacking` false))
    (:`OnInterrupted`
      (goto _label))
    (:`OnNotifyBegin`
      (switch `name` _notifyname
        (:`Fire`
          (`/Game/Dymanic/Attack-DamageSystem/Attacks/BPC_Attacks.MagicSpell` (`self.BPC_Attacks`) (`KismetMathLibrary.MakeTransform` (`SceneComponent.GetSocketLocation` (`self.Mesh`) "RightHand")) AttackTarget (make `/Game/Dymanic/Attack-DamageSystem/DamageSystem/S_DamageInfo` 20.0 "NewEnumerator2")))))))

(fn `GetIdealRange`
  (returns (AttackRadius :type "Float (double-precision)") (DefendRadius :type "Float (double-precision)"))
  (return 500.0 700.0))

(fn `SetMovementSpeed`
  (params (Speed :type "/Game/Dymanic/BluePrints/Enemies/AI/Enums/E_MovementSpeed Enum" :default "NewEnumerator0"))
  (returns (SpeedValue :type "Float (double-precision)"))
  (return (select `/Game/Dymanic/BluePrints/Enemies/AI/Enums/E_MovementSpeed` Speed :`NewEnumerator1` 150.0 :`NewEnumerator2` 250.0 :`NewEnumerator3` 400.0)))

(fn `UserConstructionScript`
  (`parent.UserConstructionScript`))