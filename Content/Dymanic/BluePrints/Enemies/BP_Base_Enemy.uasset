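; Base enemy character that pairs a damage system component with an AIC_Enemy_Base controller and a health bar widget.
; Hit responses freeze the AI for a reaction montage, then set it attacking the damage causer; death stops AI logic and ragdolls the mesh.
; Accessor functions forward health and damage calls to the component and supply patrol route, combat ranges and movement speed tiers.
; Jumps launch the character along a suggested projectile arc toward a raised destination.
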(event `self.ReceiveBeginPlay`
  (bind _asaic_enemy_base (cast `/Game/Dymanic/BluePrints/Enemies/AI/AIC_Enemy_Base` (`AIBlueprintHelperLibrary.GetAIController` self)))
  (set `self.AICEnemyBase` _asaic_enemy_base)
  (bind _returnvalue (`|CreateWidget` "/Game/Dymanic/DamageSystem/W_HealthBar.W_HealthBar_C" null self))
  (`WidgetComponent.SetWidget` (`self.HealthBar`) _returnvalue)
  (add `/Game/Dymanic/DamageSystem/BPC_DamageSystem.OnDeath` (`self.BPC_DamageSystem`) (`|CreateDelegate` :!event `Die`))
  (add `/Game/Dymanic/DamageSystem/BPC_DamageSystem.OnDamageResponse` (`self.BPC_DamageSystem`) (`|CreateDelegate` :!event `HitResponse`)))

(event `Die`
  (bind _mesh (`self.Mesh`))
  ;[0 0 0] Death
  (`PrimitiveComponent.SetCollisionEnabled` (`self.CapsuleComponent`) "NoCollision")
  (`PrimitiveComponent.SetSimulatePhysics` _mesh true)
  (`PrimitiveComponent.SetCollisionEnabled` _mesh "QueryAndPhysics")
  (`BrainComponent.StopLogic` (`AIController.BrainComponent` (`self.AICEnemyBase`)) "")
  (`/Game/Dymanic/BluePrints/Enemies/AI/AIC_Enemy_Base.SetStateAsDead` (`self.AICEnemyBase`)))

(event `HitResponse`
  (params (DamageResponse :type "/Game/Dymanic/DamageSystem/E_DamageResponse Enum" :default "NewEnumerator0") (DamageCauser :type "Actor Object Reference"))
  (`MovementComponent.StopMovementImmediately` (`self.CharacterMovement`))
  (`/Game/Dymanic/BluePrints/Enemies/AI/AIC_Enemy_Base.SetStateAsFrozen` (`self.AICEnemyBase`))
  (`|PlayMontage` (`self.Mesh`) (`self.HitReactionMontage`)
    (:`OnCompleted`
      _)
    (:`OnInterrupted`
      _))
  (`/Game/Dymanic/BluePrints/Enemies/AI/AIC_Enemy_Base.Set State as Attacking` (`self.AICEnemyBase`) DamageCauser true))

(event `/Game/Dymanic/BluePrints/Enemies/AI/BPI_EnemyAI.JumpDestination`
  (params (Destination :type "Vector Structure"))
  (bind _outlaunchvelocity (`GameplayStatics.SuggestProjectileVelocity_CustomArc` (`self.K2_GetActorLocation`) (`KismetMathLibrary.MakeVector` (.x Destination) (.y Destination) (+ (.z Destination) 250.0))))
  (`self.LaunchCharacter` _outlaunchvelocity true true))

(fn `GetCurrentHealth`
  (returns (Health :type "Float (double-precision)"))
  (return (`/Game/Dymanic/DamageSystem/BPC_DamageSystem.Health` (`self.BPC_DamageSystem`))))

(fn `GetIdealRange`
  (returns (AttackRadius :type "Float (double-precision)") (DefendRadius :type "Float (double-precision)"))
  (return 150.0 350.0))

(fn `GetMaxHealth`
  (returns (MaxHealth :type "Float (double-precision)"))
  (return (`/Game/Dymanic/DamageSystem/BPC_DamageSystem.MaxHealth` (`self.BPC_DamageSystem`))))

(fn `GetPatrolRoute`
  (returns (PatrolRoute :type "/Game/Dymanic/BluePrints/Enemies/AI/BP_PatrolRoute Object Reference"))
  (return (`self.PatrolRoute`)))

(fn `Heal`
  (params (Amount :type "Float (double-precision)"))
  (returns (NewHealth :type "Float (double-precision)"))
  (bind _newhealth (`/Game/Dymanic/DamageSystem/BPC_DamageSystem.Heal` (`self.BPC_DamageSystem`) Amount))
  (return _newhealth))

(fn `IsDead`
  (returns (Dead :type Boolean))
  (return (`/Game/Dymanic/DamageSystem/BPC_DamageSystem.IsDead` (`self.BPC_DamageSystem`))))

(fn `SetMovementSpeed`
  (params (Speed :type "/Game/Dymanic/BluePrints/Enemies/AI/Enums/E_MovementSpeed Enum" :default "NewEnumerator0"))
  (returns (SpeedValue :type "Float (double-precision)"))
  (bind _output_get (set `CharacterMovementComponent.MaxWalkSpeed` (select `/Game/Dymanic/BluePrints/Enemies/AI/Enums/E_MovementSpeed` Speed :`NewEnumerator1` 100.0 :`NewEnumerator2` 300.0 :`NewEnumerator3` 500.0 :!type "Float (single-precision)") (`self.CharacterMovement`)))
  (return _output_get))

(fn `TakeDamage`
  (params (DamageInfo :type "/Game/Dymanic/DamageSystem/S_DamageInfo Structure") (`Damage Casuer` :type "Actor Object Reference"))
  (returns (WasDamaged :type Boolean))
  (bind _wasdamaged (`/Game/Dymanic/DamageSystem/BPC_DamageSystem.TakeDamage` (`self.BPC_DamageSystem`) DamageInfo `Damage Casuer`))
  (return _wasdamaged))

(fn `UserConstructionScript`
  (bind _bpc_damagesystem (`self.BPC_DamageSystem`))
  (set `/Game/Dymanic/DamageSystem/BPC_DamageSystem.MaxHealth` 100.0 _bpc_damagesystem)
  (set `/Game/Dymanic/DamageSystem/BPC_DamageSystem.Health` 100.0 _bpc_damagesystem))