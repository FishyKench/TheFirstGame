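; Ranged enemy Blueprint that spawns a rifle on BeginPlay, attaches it to the hand socket and fires at its AI controller's attack target.
; Attack plays the fire montage, blocking interruption through the damage system until it ends, then signals attack end.
; A montage notify runs a debug-drawn visibility line trace and sends fixed damage only if nothing blocks it.
; It also supplies walk speeds per movement state and ideal attack and defend ranges.
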(event `self.ReceiveBeginPlay`
  (`|ExecutionSequence`
    (:`then_0`
      (`parent.ReceiveBeginPlay`))
    (:`then_1`
      (bind _returnvalue (`|SpawnActorFromClass` "/Game/Dymanic/weapons/Meshes/BP_Rifle.BP_Rifle_C" (`self.GetTransform`) "Undefined" "MultiplyWithRoot" null null))
      (bind _output_get (set `self.WeaponActor` _returnvalue))
      (`self.K2_AttachToComponent` _output_get (`self.Mesh`) "hand_r_rifle_socket" "SnapToTarget" "SnapToTarget" "SnapToTarget" true))
    (:`then_2`
      (`parent.ReceiveBeginPlay`))))

(event `/Game/Dymanic/BluePrints/Enemies/AI/BPI_EnemyAI.Attack`
  (bind _notifyname (`|PlayMontage` (`self.Mesh`) "/Game/Dymanic/BluePrints/Enemies/AI/Animations_Imported/Rifle/Montage_Rifle_Fire.Montage_Rifle_Fire")
    (:`then`
      (set `/Game/Dymanic/DamageSystem/BPC_DamageSystem.IsInterruptible` false (`self.BPC_DamageSystem`)))
    (:`OnCompleted`
      (`self.OnAttackEnd` :!label _label)
      (set `/Game/Dymanic/DamageSystem/BPC_DamageSystem.IsInterruptible` true (`self.BPC_DamageSystem`)))
    (:`OnInterrupted`
      (goto _label))
    (:`OnNotifyBegin`
      (switch `name` _notifyname
        (:`Fire`
          (bind _asaic_enemy_base (cast `/Game/Dymanic/BluePrints/Enemies/AI/AIC_Enemy_Base` (`AIBlueprintHelperLibrary.GetAIController` self)))
          (bind _attacktarget (`/Game/Dymanic/BluePrints/Enemies/AI/AIC_Enemy_Base.AttackTarget` _asaic_enemy_base)
            (:`then`
              (bind (_outhit _returnvalue) (`KismetSystemLibrary.LineTraceSingle` :`Start` (`self.K2_GetActorLocation`) :`End` (`self.K2_GetActorLocation` _attacktarget) :`TraceChannel` "TraceTypeQuery1" :`DrawDebugType` "ForDuration"))
              (if (not _returnvalue)
                (message `/Game/Dymanic/DamageSystem/BPI_Damagable.TakeDamage` _attacktarget (make `/Game/Dymanic/DamageSystem/S_DamageInfo` 20.0 "NewEnumerator2"))))
            (:`else`)))))))

(fn `GetIdealRange`
  (returns (AttackRadius :type "Float (double-precision)") (DefendRadius :type "Float (double-precision)"))
  (return 600.0 600.0))

(fn `SetMovementSpeed`
  (params (Speed :type "/Game/Dymanic/BluePrints/Enemies/AI/Enums/E_MovementSpeed Enum" :default "NewEnumerator0"))
  (returns (SpeedValue :type "Float (double-precision)"))
  (bind _output_get (set `CharacterMovementComponent.MaxWalkSpeed` (select `/Game/Dymanic/BluePrints/Enemies/AI/Enums/E_MovementSpeed` Speed :`NewEnumerator1` 200.0 :`NewEnumerator2` 300.0 :`NewEnumerator3` 500.0 :!type "Float (single-precision)") (`self.CharacterMovement`)))
  (return _output_get))

(fn `UserConstructionScript`
  (`parent.UserConstructionScript`))