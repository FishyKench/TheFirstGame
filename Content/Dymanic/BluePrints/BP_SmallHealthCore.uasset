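; BP_SmallHealthCore is a pickup that gives the player a small heal when touched.
; On BeginPlay it caches the player character as a BP_Player reference.
; When that player overlaps its collision sphere, it overwrites the player's HealAmountOnKill with SmallHeal, calls HealPlayerOnKill to reuse the heal-on-kill logic, then destroys itself.
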(event `self.ReceiveBeginPlay`
  (bind _asbp_player (cast `/Game/Dymanic/BluePrints/BP_Player` (`GameplayStatics.GetPlayerCharacter` 0)))
  (set `self.Player` _asbp_player))

(event `self.SphereCollision.OnComponentBeginOverlap`
  (params (OverlappedComponent :type "PrimitiveComponent Object Reference") (OtherActor :type "Actor Object Reference") (OtherComp :type "PrimitiveComponent Object Reference") (OtherBodyIndex :type Integer) (bFromSweep :type Boolean) (SweepResult :type "HitResult Structure (by ref)"))
  (if (== OtherActor (`self.Player`))
    (set `/Game/Dymanic/BluePrints/BP_Player.HealAmountOnKill` (`self.SmallHeal`) (`self.Player`))
    (`/Game/Dymanic/BluePrints/BP_Player.HealPlayerOnKill` (`self.Player`))
    (`self.K2_DestroyActor`)))

(fn `UserConstructionScript`)