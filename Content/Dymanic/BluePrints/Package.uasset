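; Package is a physics actor that launches itself on BeginPlay and disappears when the first-person player character touches it.
; ThrowPackage applies a random-strength impulse to the Cube, equal on all three axes and randomly all positive or all negative through LeftForce and RightForce, then randomizes its rotation.
; BeginPlay also caches the player character, which the Box overlap compares against before destroying the actor.
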(event `ThrowPackage`
  (bind _returnvalue (`KismetMathLibrary.RandomFloatInRange` 35000.0 50000.0))
  ;[0 0 0] ThrowPackage
  (`|ExecutionSequence`
    (:`then_0`
      (if (`KismetMathLibrary.RandomBool`)
        (bind _outputaxis (`self.LeftForce` _returnvalue)
          (:`NewParam2`
            (`PrimitiveComponent.AddImpulse` (`self.Cube`) (`KismetMathLibrary.MakeVector` _outputaxis _outputaxis _outputaxis) "None" false)))
        (else
          (bind _outputaxis_2 (`self.RightForce` _returnvalue)
            (:`NewParam2`
              (`PrimitiveComponent.AddImpulse` (`self.Cube`) (`KismetMathLibrary.MakeVector` _outputaxis_2 _outputaxis_2 _outputaxis_2) "None" false))))))
    (:`then_1`
      (`SceneComponent.K2_SetWorldRotation` (`self.Cube`) (`KismetMathLibrary.RandomRotator` false) false false))))

(event `self.Box.OnComponentBeginOverlap`
  (params (OverlappedComponent :type "PrimitiveComponent Object Reference") (OtherActor :type "Actor Object Reference") (OtherComp :type "PrimitiveComponent Object Reference") (OtherBodyIndex :type Integer) (bFromSweep :type Boolean) (SweepResult :type "HitResult Structure (by ref)"))
  ;[0 0 0] OnPlayerCollision
  (if (== OtherActor (`self.As BP First Person Character`))
    (`self.K2_DestroyActor`)))

(event `self.ReceiveBeginPlay`
  ;[0 0 0] EventBeginPlay
  (`|ExecutionSequence`
    (:`then_0`
      (bind _asbp_first_person_character (cast `/Game/Dymanic/FirstPerson/Blueprints/BP_FirstPersonCharacter` (`GameplayStatics.GetPlayerCharacter` 0)))
      (set `self.As BP First Person Character` _asbp_first_person_character))
    (:`then_1`
      (`self.ThrowPackage`))))

(fn `UserConstructionScript`)