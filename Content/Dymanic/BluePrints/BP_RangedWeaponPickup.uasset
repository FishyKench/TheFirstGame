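; BP_RangedWeaponPickup is a world pickup that gives the player a ranged weapon when they overlap its sphere.
; The construction script previews the configured mesh and material on the Weapon component.
; BeginPlay caches the BP_Player, and on overlap with that player it copies the mesh, material, attack range, damage and name onto the player, then calls SwitchRangedWeapon.
; The pickup is not destroyed or disabled afterwards.
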(event `self.ReceiveBeginPlay`
  (bind _asbp_player (cast `/Game/Dymanic/BluePrints/BP_Player` (`GameplayStatics.GetPlayerCharacter` 0)))
  (set `self.Player` _asbp_player))

(event `self.Sphere.OnComponentBeginOverlap`
  (params (OverlappedComponent :type "PrimitiveComponent Object Reference") (OtherActor :type "Actor Object Reference") (OtherComp :type "PrimitiveComponent Object Reference") (OtherBodyIndex :type Integer) (bFromSweep :type Boolean) (SweepResult :type "HitResult Structure (by ref)"))
  (bind _player (`self.Player`))
  (bind _rangedweapon (`/Game/Dymanic/BluePrints/BP_Player.RangedWeapon` (`self.Player`)))
  (if (== OtherActor (`self.Player`))
    (`StaticMeshComponent.SetStaticMesh` _rangedweapon (`self.WeaponMesh`))
    (`PrimitiveComponent.SetMaterial` _rangedweapon 0 (`self.WeaponMaterial`))
    (set `/Game/Dymanic/BluePrints/BP_Player.AttackRange(Range)` (`self.AttackRange`) _player)
    (set `/Game/Dymanic/BluePrints/BP_Player.WeaponDamage(Ranged)` (`self.WeaponDamage`) _player)
    (set `/Game/Dymanic/BluePrints/BP_Player.RangedWeaponName` (`self.WeaponName`) _player)
    (`/Game/Dymanic/BluePrints/BP_Player.SwitchRangedWeapon` _player)))

(fn `UserConstructionScript`
  (bind _weapon (`self.Weapon`))
  (`StaticMeshComponent.SetStaticMesh` _weapon (`self.WeaponMesh`))
  (`PrimitiveComponent.SetMaterial` _weapon 0 (`self.WeaponMaterial`)))