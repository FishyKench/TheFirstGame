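; Upgrade shrine actor that opens a wave shop widget, created hidden at BeginPlay, when the player interacts with it.
; While the player is inside its box, a looping timer line-traces from the first-person camera and swaps to a highlight material when aimed at.
; Interacting while aimed toggles the shop.
; Opening stops the trace timer and switches to UI-only input; closing hides the widget and restores game-only input.
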(event `self.ReceiveBeginPlay`
  ;[0 0 0] Create the Shop widget (UI) in "Begin play" but hide it
  (bind _returnvalue (`|CreateWidget` "/Game/Dymanic/BluePrints/UI/WB_WaveShop.WB_WaveShop_C"))
  (bind _output_get (set `self.ShopUI` _returnvalue))
  (`UserWidget.AddToViewport` _output_get 0)
  (`Widget.SetVisibility` (`self.ShopUI`) "Hidden")
  (set `/Game/Dymanic/BluePrints/UI/WB_WaveShop.BP_UpgradeShrine` self (`self.ShopUI`)))

(event `self.Box.OnComponentEndOverlap`
  (params (OverlappedComponent :type "PrimitiveComponent Object Reference") (OtherActor :type "Actor Object Reference") (OtherComp :type "PrimitiveComponent Object Reference") (OtherBodyIndex :type Integer))
  ;[0 0 0] if away from shrine stop checking
  (cast `/Game/Dymanic/BluePrints/BP_Player` OtherActor)
  (`KismetSystemLibrary.K2_ClearAndInvalidateTimerHandle` (`self.LinecastTimer`)))

(event `self.Box.OnComponentBeginOverlap`
  (params (OverlappedComponent :type "PrimitiveComponent Object Reference") (OtherActor :type "Actor Object Reference") (OtherComp :type "PrimitiveComponent Object Reference") (OtherBodyIndex :type Integer) (bFromSweep :type Boolean) (SweepResult :type "HitResult Structure (by ref)"))
  ;[0 0 0] if close to shrine check what player is looking at
  (bind _asbp_player (cast `/Game/Dymanic/BluePrints/BP_Player` OtherActor))
  (set `self.BP_Player` _asbp_player)
  (bind _returnvalue (`KismetSystemLibrary.K2_SetTimerDelegate` (delegate `LinecastFromPlayer`) 0.1 true))
  (set `self.LinecastTimer` _returnvalue))

(event `CloseShop`
  ;[0 0 0] If Shop = Open -> Close
  (set `self.ShopOpen?` false)
  (`Widget.SetVisibility` (`self.ShopUI`) "Hidden")
  (`WidgetBlueprintLibrary.SetInputMode_GameOnly` (`GameplayStatics.GetPlayerController` 0)))

(event `LinecastFromPlayer`
  (bind _firstpersoncamera (`/Game/Dymanic/BluePrints/BP_Player.FirstPersonCamera` (`self.BP_Player`)))
  (bind _returnvalue (`SceneComponent.K2_GetComponentLocation` _firstpersoncamera))
  ;[0 0 0] Check what player is looking at
  (bind _outhit (`KismetSystemLibrary.LineTraceSingle` :`Start` _returnvalue :`End` (+ _returnvalue (* (`KismetMathLibrary.GetForwardVector` (`SceneComponent.K2_GetComponentRotation` _firstpersoncamera)) 500.0)) :`TraceChannel` "TraceTypeQuery1" :`DrawDebugType` "ForOneFrame" :`bIgnoreSelf` false))
  ;[0 0 0] Highlight shrine if player looks at it
  (if (== (`.HitActor` (`GameplayStatics.BreakHitResult` _outhit)) self)
    (`PrimitiveComponent.SetMaterial` (`self.ShrineMesh`) 0 (`self.HighlightMaterial`))
    ;[0 0 0] Check if looking at + interacted with shrine
    (if (== (`/Game/Dymanic/BluePrints/BP_Player.InteractedWithActor` (`self.BP_Player`)) self)
      (if (`self.ShopOpen?`)
        (`self.CloseShop`)
        (else
          (`self.OpenShop`))))
    (else
      (`PrimitiveComponent.SetMaterial` (`self.ShrineMesh`) 0 (`self.DefaultMaterial`)))))

(event `OpenShop`
  (bind _shopui (`self.ShopUI`))
  ;[0 0 0] If Shop = Closed -> Open & stop checking (linecasting)
  (bind _output_get (set `self.ShopOpen?` true))
  (`KismetSystemLibrary.K2_ClearAndInvalidateTimerHandle` (`self.LinecastTimer`))
  (`KismetSystemLibrary.PrintString` (`KismetStringLibrary.Conv_BoolToString` _output_get))
  (`Widget.SetVisibility` _shopui "Visible")
  (`WidgetBlueprintLibrary.SetInputMode_UIOnlyEx` (`GameplayStatics.GetPlayerController` 0) _shopui)
  (set `/Game/Dymanic/BluePrints/BP_Player.InteractedWithActor` null (`self.BP_Player`)))

(fn `UserConstructionScript`)