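; Upgrade shrine actor that offers three randomly rolled upgrade names and highlights when the player looks at it.
; On BeginPlay, RollPoolUpgrade fills three texts from the available names, but removes and prints separately re-rolled picks, so duplicates can appear.
; While BP_Player overlaps the box, a looping timer line-traces from the first-person camera to swap the mesh material.
; The interaction check is an empty stub.
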(event `self.ReceiveBeginPlay`
  (`self.StartShrineLogic`))

(event `StartShrineLogic`
  (`self.RollUpgrades`))

(event `RollUpgrades`
  (`self.RollPoolUpgrade` (`self.P1UpgradeName`)
    (:`ExecOut`
      (`self.RollPoolUpgrade` (`self.P2UpgradeName`)
        (:`ExecOut`
          (`self.RollPoolUpgrade` (`self.P3UpgradeName`)))))))

(event `self.Box.OnComponentEndOverlap`
  (params (OverlappedComponent :type "PrimitiveComponent Object Reference") (OtherActor :type "Actor Object Reference") (OtherComp :type "PrimitiveComponent Object Reference") (OtherBodyIndex :type Integer))
  ;[0 0 0] if away from shrine stop checking
  (cast `/Game/Dymanic/BluePrints/BP_Player` OtherActor)
  (`KismetSystemLibrary.K2_ClearAndInvalidateTimerHandle` (`self.LinecastTimer`)))

(event `self.Box.OnComponentBeginOverlap`
  (params (OverlappedComponent :type "PrimitiveComponent Object Reference") (OtherActor :type "Actor Object Reference") (OtherComp :type "PrimitiveComponent Object Reference") (OtherBodyIndex :type Integer) (bFromSweep :type Boolean) (SweepResult :type "HitResult Structure (by ref)"))
  ;[0 0 0] if close to shrine check what player is looking at
  (bind _asbp_player (cast `/Game/Dymanic/BluePrints/BP_Player` OtherActor))
  (set `self.BP_Player` _asbp_player)
  (bind _returnvalue (`KismetSystemLibrary.K2_SetTimerDelegate` (delegate `LinecastFromPlayer`) 0.1 true))
  (set `self.LinecastTimer` _returnvalue))

(event `LinecastFromPlayer`
  (bind _firstpersoncamera (`/Game/Dymanic/BluePrints/BP_Player.FirstPersonCamera` (`self.BP_Player`)))
  (bind _returnvalue (`SceneComponent.K2_GetComponentLocation` _firstpersoncamera))
  ;[0 0 0] Check what player is looking at
  (bind _outhit (`KismetSystemLibrary.LineTraceSingle` :`Start` _returnvalue :`End` (+ _returnvalue (* (`KismetMathLibrary.GetForwardVector` (`SceneComponent.K2_GetComponentRotation` _firstpersoncamera)) 500.0)) :`TraceChannel` "TraceTypeQuery1" :`DrawDebugType` "ForOneFrame" :`bIgnoreSelf` false))
  ;[0 0 0] Highlight shrine if player looks at it
  (if (== (`.HitActor` (`GameplayStatics.BreakHitResult` _outhit)) self)
    (`PrimitiveComponent.SetMaterial` (`self.ShrineMesh`) 0 (`self.HighlightMaterial`))
    ;[0 0 0] Check if looking at + interacted with shrine
    (if (== (`/Game/Dymanic/BluePrints/BP_Player.InteractedWithActor` (`self.BP_Player`)) self)
      (if true
        _))
    (else
      (`PrimitiveComponent.SetMaterial` (`self.ShrineMesh`) 0 (`self.DefaultMaterial`)))))

(fn `UserConstructionScript`)