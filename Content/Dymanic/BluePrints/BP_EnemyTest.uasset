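; BP_EnemyTest is a test enemy actor that takes damage and drops a HealthCore when it dies.
; AnyDamage subtracts from Health, and at zero or below it clamps Health, spawns the HealthCore, then destroys itself after a very short Delay.
; The drop's spawn location comes from the Cylinder component's relative location rather than a world location.
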(event `self.ReceiveAnyDamage`
  (params (Damage :type "Float (single-precision)") (DamageType :type "DamageType Object Reference") (InstigatedBy :type "Controller Object Reference") (DamageCauser :type "Actor Object Reference"))
  (bind _output_get (set `self.Health` (- (`self.Health`) Damage)))
  (if (<= _output_get 0.0)
    (set `self.Health` 0.0)
    (`|SpawnActorFromClass` (`self.HealthCore`) (`KismetMathLibrary.MakeTransform` (`SceneComponent.RelativeLocation` (`self.Cylinder`))) "Undefined" "MultiplyWithRoot" null null)
    (`KismetSystemLibrary.Delay` 0.001)
    (`self.K2_DestroyActor`)))

(fn `UserConstructionScript`)